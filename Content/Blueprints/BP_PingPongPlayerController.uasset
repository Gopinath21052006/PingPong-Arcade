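; Player controller for a ping pong game that handles keyboard and mapped input for match flow and paddle movement.
; On BeginPlay it sets game-only input, hides the cursor and caches the BP_PingPongGameMode.
; Keys and actions forward two-player toggle, pause, restart, 1P/2P start and home menu to the game mode, while quit exits directly.
; Two movement axes are stored in variables for both players, with no pawn movement done here.
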(event EventBeginPlay
  (Input|SetInputModeGameOnly self false)
  (Variables|Default|SetbShowMouseCursor false)
  (bind _asbp_ping_pong_game_mode (Utilities|Casting|CastToBP_PingPongGameMode (Game|GetGameMode)))
  (Variables|Default|SetGameModeRef _asbp_ping_pong_game_mode))

(event EventTick
  (params (DeltaSeconds :type Float%20%28single-precision%29)))

(event Input|ActionEvents|InputActionSelect1P
  (params (Key :type Key%20Structure))
  (:Pressed
    (Default|StartMatch1P (Variables|Default|GetGameModeRef))))

(event Input|ActionEvents|InputActionQuit
  (params (Key :type Key%20Structure))
  (:Pressed
    (Game|QuitGame 0 "Quit" false)))

(event Input|ActionEvents|InputActionSelect2P
  (params (Key :type Key%20Structure))
  (:Pressed
    (Default|StartMatch2P (Variables|Default|GetGameModeRef))))

(event Input|ActionEvents|InputActionHomeMenu
  (params (Key :type Key%20Structure))
  (:Pressed
    (Default|ReturntoHome (Variables|Default|GetGameModeRef))))

(event Input|AxisEvents|InputAxisMovePlayer2
  (params (AxisValue :type Float%20%28single-precision%29))
  (Variables|Default|SetMovePlayer2Axis AxisValue))

(event Input|AxisEvents|InputAxisMovePlayer
  (params (AxisValue :type Float%20%28single-precision%29))
  (Variables|Default|SetMoveAxis AxisValue))

(event Input|KeyboardEvents|Tab
  (params (Key :type Key%20Structure))
  (:Pressed
    (Default|Toggle2Player (Variables|Default|GetGameModeRef))))

(event Input|KeyboardEvents|P
  (params (Key :type Key%20Structure))
  (:Pressed
    (Default|TogglePause (Variables|Default|GetGameModeRef))))

(event Input|KeyboardEvents|SpaceBar
  (params (Key :type Key%20Structure))
  (:Pressed
    (Default|RestartMatch (Variables|Default|GetGameModeRef))))

(event Input|KeyboardEvents|Up
  (params (Key :type Key%20Structure)))

(event Input|KeyboardEvents|Down
  (params (Key :type Key%20Structure)))

(event Input|KeyboardEvents|T
  (params (Key :type Key%20Structure))
  (:Pressed
    (Default|Toggle2Player (Variables|Default|GetGameModeRef))))

(fn ConstructionScript)